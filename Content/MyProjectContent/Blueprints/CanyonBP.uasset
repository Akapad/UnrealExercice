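; CanyonBP is a cannon-style turret that aims at player 0's pawn and fires continuously from BeginPlay.
; Tick sets yaw on BaseSM and CanyonSM, plus pitch on CanyonSM, using constant-speed interpolation toward a look-at rotation.
; Yaw interpolates from the actor's rotation, while pitch interpolates from the barrel's own.
; ShootEvt re-calls itself after random delays, spawning a scaled-down actor at ShootLocation with an impulse and slightly randomised forward direction.
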(event `self.ReceiveBeginPlay`
  (`self.ShootEvt`))

(event `ShootEvt`
  (bind _canyonsm (`self.CanyonSM`))
  (`KismetSystemLibrary.Delay` (`KismetMathLibrary.RandomFloatInRange` 0.1 2.0))
  (`|SpawnActorFromClass` null (`KismetMathLibrary.MakeTransform` (`SceneComponent.K2_GetComponentLocation` (`self.ShootLocation`)) (`SceneComponent.K2_GetComponentRotation` _canyonsm) (0.1 0.1 0.1)) "AlwaysSpawn" "OverrideRootScale" null (+ (`SceneComponent.GetForwardVector` _canyonsm) (* (`KismetMathLibrary.RandomUnitVector`) 0.1)) 2000.0 null)
  (`self.ShootEvt`))

(event `self.ReceiveTick`
  (params (DeltaSeconds :type "Float (single-precision)"))
  (bind _returnvalue (`KismetMathLibrary.FInterpTo_Constant` (.yaw (`self.K2_GetActorRotation`)) (.yaw (`KismetMathLibrary.FindLookAtRotation` (`SceneComponent.K2_GetComponentLocation` (`self.CanyonSM`)) (`self.K2_GetActorLocation` (`GameplayStatics.GetPlayerPawn` 0)))) DeltaSeconds 30.0))
  (`SceneComponent.K2_SetWorldRotation` (`self.BaseSM`) (`KismetMathLibrary.MakeRotator` 0.0 0.0 _returnvalue) false false)
  (`SceneComponent.K2_SetWorldRotation` (`self.CanyonSM`) (`KismetMathLibrary.MakeRotator` 0.0 (`KismetMathLibrary.FInterpTo_Constant` (.pitch (`SceneComponent.K2_GetComponentRotation` (`self.CanyonSM`))) (.pitch (`KismetMathLibrary.FindLookAtRotation` (`SceneComponent.K2_GetComponentLocation` (`self.CanyonSM`)) (`self.K2_GetActorLocation` (`GameplayStatics.GetPlayerPawn` 0)))) (`GameplayStatics.GetWorldDeltaSeconds`) 40.0) _returnvalue) false false))

(fn `UserConstructionScript`)