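; Moving platform actor that slides its mesh along the actor's forward axis and glows while a specific type of actor overlaps its box.
; BeginPlay stores the start location and fires MovementEvt, whose timeline curve scales the Offset distance to set the mesh position without sweeping.
; The construction script creates a dynamic material for the mesh, and box overlap begin and end events switch its "Brillo" brightness parameter on and off.
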(event `MovementEvt`
  (bind (_direction _offset) (`Timeline|MovementTL` :!via `PlayFromStart`)
    (:`Update`
      (`SceneComponent.K2_SetWorldLocation` (`self.PlatformSM`) (+ (* (`self.GetActorForwardVector`) (* _offset (`self.Offset`))) (`self.InitPos`)) false false))))

(event `self.ReceiveBeginPlay`
  (set `self.InitPos` (`self.K2_GetActorLocation`))
  (`self.MovementEvt`))

(event `self.Box.OnComponentBeginOverlap`
  (params (OverlappedComponent :type "PrimitiveComponent Object Reference") (OtherActor :type "Actor Object Reference") (OtherComp :type "PrimitiveComponent Object Reference") (OtherBodyIndex :type Integer) (bFromSweep :type Boolean) (SweepResult :type "HitResult Structure (by ref)"))
  (cast `` OtherActor)
  (`MaterialInstanceDynamic.SetScalarParameterValue` (`self.Material`) "Brillo" 500.0))

(event `self.Box.OnComponentEndOverlap`
  (params (OverlappedComponent :type "PrimitiveComponent Object Reference") (OtherActor :type "Actor Object Reference") (OtherComp :type "PrimitiveComponent Object Reference") (OtherBodyIndex :type Integer))
  (cast `` OtherActor)
  (`MaterialInstanceDynamic.SetScalarParameterValue` (`self.Material`) "Brillo" 0.0))

(fn `UserConstructionScript`
  (bind _returnvalue (`KismetMaterialLibrary.CreateDynamicMaterialInstance` null))
  (bind _output_get (set `self.Material` _returnvalue))
  (`PrimitiveComponent.SetMaterial` (`self.PlatformSM`) 0 _output_get))